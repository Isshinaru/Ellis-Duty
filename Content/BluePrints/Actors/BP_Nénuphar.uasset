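; BP_Nénuphar is a lily pad platform actor that moves down after an actor overlaps it, then returns to its original position.
; BeginPlay stores the Cube's relative start position and an end position offset vertically by MoveZ.
; Overlap triggers a delay and timed MoveComponentTo toward the end, then sets Down.
; Tick polls Down to run the same delayed move back and clear the flag.
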(event `self.ReceiveBeginPlay`
  (bind (_posstart_x _posstart_y _posstart_z) (`KismetMathLibrary.BreakVector` (`self.PosStart`)))
  (set `self.PosStart` (`SceneComponent.RelativeLocation` (`self.Cube`)))
  (set `self.PosEnd` (`KismetMathLibrary.MakeVector` _posstart_x _posstart_y (+ _posstart_z (`self.MoveZ`)))))

(event `self.ReceiveActorBeginOverlap`
  (params (OtherActor :type "Actor Object Reference"))
  (if (not (`self.Down`))
    (`KismetSystemLibrary.Delay` (`self.TimeBeforeDown`))
    (`KismetSystemLibrary.MoveComponentTo` (`self.Cube`) (`self.PosEnd`) (struct) false false (`self.TimeForDown`))
    (set `self.Down` true)))

(event `self.ReceiveTick`
  (params (DeltaSeconds :type "Float (single-precision)"))
  (if (`self.Down`)
    (`KismetSystemLibrary.Delay` (`self.TimeBeforeDown`))
    (`KismetSystemLibrary.MoveComponentTo` (`self.Cube`) (`self.PosStart`) (struct) false false (`self.TimeForDown`))
    (set `self.Down` false)))

(fn `UserConstructionScript`)