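; BP_Arbre is a tree actor whose trunk (Tronc) moves to an end pose when a MainCharacter with enough Mana overlaps it.
; BeginPlay moves the trunk to the StartPos pose.
; A qualifying overlap calls RegenElem on the character, waits TimeBeforeUp, then uses MoveComponentTo to move the trunk to EndPos over TimeForUp.
; Debug prints remain in the overlap logic, and nothing moves the trunk back afterwards.
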(event `self.ReceiveBeginPlay`
  (bind (_startpos_location _startpos_rotation) (`KismetMathLibrary.BreakTransform` (`self.StartPos`)))
  (`KismetSystemLibrary.MoveComponentTo` (`self.Tronc`) _startpos_location _startpos_rotation))

(event `self.ReceiveActorBeginOverlap`
  (params (OtherActor :type "Actor Object Reference"))
  (bind (_endpos_location _endpos_rotation) (`KismetMathLibrary.BreakTransform` (`self.EndPos`)))
  (`KismetSystemLibrary.PrintString` "tenta")
  (bind _asmain_character (cast `/Game/BluePrints/MainCharacter` OtherActor))
  (if (>= (`/Game/BluePrints/MainCharacter.Mana` _asmain_character) 1.0)
    (`KismetSystemLibrary.PrintString` "clean")
    (`/Game/BluePrints/MainCharacter.Regen Elem` _asmain_character)
    (`KismetSystemLibrary.Delay` (`self.TimeBeforeUp`))
    (`KismetSystemLibrary.MoveComponentTo` (`self.Tronc`) _endpos_location _endpos_rotation false false (`self.TimeForUp`))))

(fn `UserConstructionScript`)