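; BP_Feuilles is a one-shot trigger actor with three leaf components that shift aside when the main character regenerates an element.
; BeginPlay caches each leaf's target by adding MoveX to its relative X position.
; On overlap, a MainCharacter with at least one Mana gets RegenElem called and the Regen flag blocks retriggering.
; After a TimeBefore delay, MoveComponentTo slides the leaves to their targets over TimeFor.
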(event `self.ReceiveBeginPlay`
  (bind (_relativelocation_x _relativelocation_y _relativelocation_z) (`KismetMathLibrary.BreakVector` (`SceneComponent.RelativeLocation` (`self.Feuille3`))))
  (bind (_relativelocation_x_2 _relativelocation_y_2 _relativelocation_z_2) (`KismetMathLibrary.BreakVector` (`SceneComponent.RelativeLocation` (`self.Feuille1`))))
  (bind (_relativelocation_x_3 _relativelocation_y_3 _relativelocation_z_3) (`KismetMathLibrary.BreakVector` (`SceneComponent.RelativeLocation` (`self.Feuille2`))))
  (set `self.MoveFeuille1` (`KismetMathLibrary.MakeVector` (+ _relativelocation_x_2 (`self.MoveX`)) _relativelocation_y_2 _relativelocation_z_2))
  (set `self.MoveFeuille2` (`KismetMathLibrary.MakeVector` (+ _relativelocation_x_3 (`self.MoveX`)) _relativelocation_y_3 _relativelocation_z_3))
  (set `self.MoveFeuille3` (`KismetMathLibrary.MakeVector` (+ _relativelocation_x (`self.MoveX`)) _relativelocation_y _relativelocation_z)))

(event `self.ReceiveActorBeginOverlap`
  (params (OtherActor :type "Actor Object Reference"))
  (if (not (`self.Regen`))
    (bind _asmain_character (cast `/Game/BluePrints/MainCharacter` OtherActor))
    (if (>= (`/Game/BluePrints/MainCharacter.Mana` _asmain_character) 1.0)
      (`/Game/BluePrints/MainCharacter.Regen Elem` _asmain_character)
      (set `self.Regen` true)
      (`KismetSystemLibrary.Delay` (`self.TimeBefore`))
      (`KismetSystemLibrary.MoveComponentTo` (`self.Feuille1`) (`self.MoveFeuille1`) (struct) false false (`self.TimeFor`))
      (`KismetSystemLibrary.MoveComponentTo` (`self.Feuille2`) (`self.MoveFeuille2`) (struct) false false (`self.TimeFor`))
      (`KismetSystemLibrary.MoveComponentTo` (`self.Feuille3`) (`self.MoveFeuille3`) (struct) false false (`self.TimeFor`)))))

(fn `UserConstructionScript`)