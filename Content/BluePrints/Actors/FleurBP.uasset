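; FleurBP is a flower actor that starts at zero scale and blooms when the player interacts with it.
; Its trigger shows Bubble prompts and opens a gate for interaction input, which requires the character can move and has enough mana.
; Success calls RegenElem, removes trigger and butterfly hint, and plays sound and shockwave particles.
; A timeline scales mesh and expanding sphere and drives particles, then updates the CompteFleur counter.
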(event `self.ReceiveBeginPlay`
  (bind _staticmesh (`self.StaticMesh`))
  (set `self.DestTransFleur` (`SceneComponent.K2_GetComponentScale` _staticmesh))
  (`SceneComponent.SetWorldScale3D` _staticmesh (0.0 0.0 0.0))
  (set `self.DestTransGrass` (`SceneComponent.K2_GetComponentScale` (`self.ParticleSystem`)))
  (`SceneComponent.K2_SetRelativeLocation` (`self.SmthHere`) (0.0 0.0 0.0) false true))

(event `Growth`
  (bind _sphere (`self.Sphere`))
  (bind _particlesystem (`self.ParticleSystem`))
  (bind (_direction _newtrack_0 _expand) (`Timeline|Timeline_0`)
    (:`Update`
      (`SceneComponent.SetWorldScale3D` (`self.StaticMesh`) (* (`self.DestTransFleur`) _newtrack_0))
      (bind _returnvalue (* _expand 100.0))
      (`SceneComponent.SetWorldScale3D` _sphere (`KismetMathLibrary.MakeVector` _returnvalue _returnvalue _returnvalue))
      (`FXSystemComponent.SetFloatParameter` _particlesystem "SinceSpawn" _newtrack_0)
      (if (not (`ActorComponent.IsActive` _particlesystem))
        (`ActorComponent.Activate` _particlesystem true)))
    (:`Finished`
      (`ActorComponent.K2_DestroyComponent` _sphere)
      (bind _foundwidgets (`WidgetBlueprintLibrary.GetAllWidgetsOfClass` "/Game/BluePrints/UIWidgets/CompteFleur.CompteFleur_C"))
      (`/Game/BluePrints/UIWidgets/CompteFleur.UpdateFleurCompte` _foundwidgets))))

(event `self.ReceiveTick`
  (params (DeltaSeconds :type "Float (single-precision)")))

(event `PartUpdate`
  (bind _poof (`self.Poof`))
  (`ActorComponent.Activate` _poof false)
  (`FXSystemComponent.SetEmitterEnable` _poof "ShockW" true)
  (`KismetSystemLibrary.Delay` 1.0)
  (`FXSystemComponent.SetEmitterEnable` _poof "ShockW" false)
  (`KismetSystemLibrary.Delay` 3.0)
  (`ActorComponent.Deactivate` _poof))

(event `InputAction|Interaction`
  (params (Key :type "Key Structure"))
  (:`Pressed`
    (if (`/Game/BluePrints/MainCharacter.CanMove` (stale `self.TriggerFleur.OnComponentBeginOverlap` _asmain_character))
      (if (>= (`/Game/BluePrints/MainCharacter.Mana` (stale `self.TriggerFleur.OnComponentBeginOverlap` _asmain_character)) 1.0)
        (`/Engine/EditorBlueprintResources/StandardMacros.Gate` true :!label _label
          (:`Exit`
            (`ActorComponent.K2_DestroyComponent` (`self.TriggerFleur`))
            (`/Game/BluePrints/MainCharacter.RegenElem` (stale `self.TriggerFleur.OnComponentBeginOverlap` _asmain_character))
            (`self.StopButterflies`)
            (for _array_element (stale `self.TriggerFleur.OnComponentBeginOverlap` _foundwidgets)
              (`/Game/BluePrints/UIWidgets/Bubble.Fade` _array_element))))
        (else
          (bind _foundwidgets (`WidgetBlueprintLibrary.GetAllWidgetsOfClass` "/Game/BluePrints/UIWidgets/Bubble.Bubble_C"))
          (for _array_element_2 _foundwidgets
            (`/Game/BluePrints/UIWidgets/Bubble.Bubulle` _array_element_2 2)))))))

(event `self.TriggerFleur.OnComponentBeginOverlap`
  (params (OverlappedComponent :type "PrimitiveComponent Object Reference") (OtherActor :type "Actor Object Reference") (OtherComp :type "PrimitiveComponent Object Reference") (OtherBodyIndex :type Integer) (bFromSweep :type Boolean) (SweepResult :type "HitResult Structure (by ref)"))
  (bind _asmain_character (cast `/Game/BluePrints/MainCharacter` OtherActor))
  (bind _foundwidgets (`WidgetBlueprintLibrary.GetAllWidgetsOfClass` "/Game/BluePrints/UIWidgets/Bubble.Bubble_C"))
  (for _array_element _foundwidgets
    (`/Game/BluePrints/UIWidgets/Bubble.Bubulle` _array_element 1))
  (`self.EnableInput` (`GameplayStatics.GetPlayerController` 0))
  (if (`self.Detecte`)
    (set `self.Detecte` false)
    (goto _label :!via `Open`)))

(event `self.TriggerFleur.OnComponentEndOverlap`
  (params (OverlappedComponent :type "PrimitiveComponent Object Reference") (OtherActor :type "Actor Object Reference") (OtherComp :type "PrimitiveComponent Object Reference") (OtherBodyIndex :type Integer))
  (cast `/Game/BluePrints/MainCharacter` OtherActor)
  (if (not (`self.Detecte`))
    (set `self.Detecte` true)
    (bind _foundwidgets (`WidgetBlueprintLibrary.GetAllWidgetsOfClass` "/Game/BluePrints/UIWidgets/Bubble.Bubble_C"))
    (for _array_element _foundwidgets
      (`/Game/BluePrints/UIWidgets/Bubble.Fade` _array_element))
    (goto _label :!via `Close`)))

(fn `StopButterflies`
  (`ActorComponent.K2_DestroyComponent` (`self.SmthHere`))
  (`AudioComponent.Play` (`self.RegenSound`) 0.0)
  (`self.PartUpdate`)
  (`self.Growth`))

(fn `UserConstructionScript`)