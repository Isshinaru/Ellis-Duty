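; Test interactable actor that lets the MainCharacter knock a cube up or down with the Interaction input while inside its Box trigger.
; Entering the box shows an E_Interaction prompt widget and opens a gate; leaving removes the widget and closes it.
; A press sets the widget's IsPressed flag, then after a short delay passes the gate to apply a vertical impulse, alternating direction via the Down flag.
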(event `InputAction|Interaction`
  (params (Key :type "Key Structure"))
  (bind _cube (`self.Cube`))
  (:`Pressed`
    (set `/Game/E_Interaction.IsPressed` true (stale `self.Box.OnComponentBeginOverlap` _returnvalue))
    (`KismetSystemLibrary.Delay` 0.2)
    (set `/Game/E_Interaction.IsPressed` true (stale `self.Box.OnComponentBeginOverlap` _returnvalue))
    (`/Engine/EditorBlueprintResources/StandardMacros.Gate` true :!label _label
      (:`Exit`
        (if (`self.Down`)
          (`PrimitiveComponent.AddImpulse` _cube (0.0 0.0 1000.0) "None" false)
          (set `self.Down` false)
          (else
            (`PrimitiveComponent.AddImpulse` _cube (0.0 0.0 -1000.0) "None" false)
            (set `self.Down` true)))))))

(event `self.Box.OnComponentBeginOverlap`
  (params (OverlappedComponent :type "PrimitiveComponent Object Reference") (OtherActor :type "Actor Object Reference") (OtherComp :type "PrimitiveComponent Object Reference") (OtherBodyIndex :type Integer) (bFromSweep :type Boolean) (SweepResult :type "HitResult Structure (by ref)"))
  (cast `/Game/BluePrints/MainCharacter` OtherActor)
  (bind _returnvalue (`|CreateWidget` "/Game/E_Interaction.E_Interaction_C"))
  (`UserWidget.AddToViewport` _returnvalue 0)
  (goto _label :!via `Open`))

(event `self.Box.OnComponentEndOverlap`
  (params (OverlappedComponent :type "PrimitiveComponent Object Reference") (OtherActor :type "Actor Object Reference") (OtherComp :type "PrimitiveComponent Object Reference") (OtherBodyIndex :type Integer))
  (cast `/Game/BluePrints/MainCharacter` OtherActor)
  (`Widget.RemoveFromParent` (stale `self.Box.OnComponentBeginOverlap` _returnvalue))
  (goto _label :!via `Close`))

(fn `UserConstructionScript`)