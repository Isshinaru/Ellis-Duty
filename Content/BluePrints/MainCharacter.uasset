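; Player character Blueprint that handles camera look, walking, running and a variable-height jump.
; Mouse-style axes yaw the controller and pitch the ToCam component within clamped limits, while movement input is scaled by a Speed value raised during Run.
; Jump applies an initial impulse, then adds a decaying per-tick impulse while held.
; Capsule hits with upward-facing normals restore the Grounded flag.
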(event `InputAxis|TurnAround`
  (params (AxisValue :type "Float (single-precision)"))
  ;[1 1 1] Camera
  (`self.AddControllerYawInput` AxisValue))

(event `InputAxis|UpAndDown`
  (params (AxisValue :type "Float (single-precision)"))
  ;[1 1 1] Camera
  (`SceneComponent.K2_SetRelativeRotation` (`self.toCam`) (`KismetMathLibrary.MakeRotator` 0.0 (`KismetMathLibrary.FClamp` (.pitch (`KismetMathLibrary.ComposeRotators` (* (struct :`Pitch` 2.0) AxisValue) (* (`SceneComponent.RelativeRotation` (`self.toCam`)) 1.0))) -70.0 70.0)) false false))

(event `InputAxis|Horizontal`
  (params (AxisValue :type "Float (single-precision)"))
  ;[1 1 1] Movements
  (`self.AddMovementInput` (`self.GetActorRightVector`) (* AxisValue (`self.Speed`))))

(event `InputAxis|Vertical`
  (params (AxisValue :type "Float (single-precision)"))
  ;[1 1 1] Movements
  (`self.AddMovementInput` (`self.GetActorForwardVector`) (* (`self.Speed`) AxisValue)))

(event `self.ReceiveTick`
  (params (DeltaSeconds :type "Float (single-precision)"))
  ;[1 1 1] Nuancier de saut
  (if (`self.Jumping`)
    (bind _output_get (set `self.JumpImpulse` (/ (`self.JumpImpulse`) 1.2)))
    (`CharacterMovementComponent.AddImpulse` (`self.CharacterMovement`) (`KismetMathLibrary.MakeVector` 0.0 0.0 _output_get) true)))

(event `InputAction|Jump`
  (params (Key :type "Key Structure"))
  ;[1 1 1] Saut
  (:`Pressed`
    (if (`self.Grounded`)
      (`CharacterMovementComponent.AddImpulse` (`self.CharacterMovement`) (0.0 0.0 100.0) true)
      (set `self.Grounded` false)
      (set `self.Jumping` true)
      (set `self.JumpImpulse` 100.0)))
  (:`Released`
    (set `self.Jumping` false)
    (set `self.JumpImpulse` 0.0)))

(event `InputAction|Run`
  (params (Key :type "Key Structure"))
  ;[1 1 1] Course
  (:`Pressed`
    (set `self.Speed` 1.0)
    ;[1 1 1] J'aime raconter n'imp dans les DebugLog
    (`KismetSystemLibrary.PrintString` "Run Forest, run"))
  (:`Released`
    (set `self.Speed` 0.5)
    (`KismetSystemLibrary.PrintString` "Et un jour, j'ai décidé d'arrêter de courrir")))

(event `self.CapsuleComponent.OnComponentHit`
  (params (HitComponent :type "PrimitiveComponent Object Reference") (OtherActor :type "Actor Object Reference") (OtherComp :type "PrimitiveComponent Object Reference") (NormalImpulse :type "Vector Structure") (Hit :type "HitResult Structure (by ref)"))
  ;[1 1 1] Reset du saut
  (if (> (.z (`.Normal` (`GameplayStatics.BreakHitResult` Hit))) 0.8)
    ;[1 1 1] J'aime raconter n'imp dans les DebugLog
    (set `self.Grounded` true)
    (`KismetSystemLibrary.PrintString` "grounded")))

(event `InputAction|Interaction`
  (params (Key :type "Key Structure")))

(fn `UserConstructionScript`)