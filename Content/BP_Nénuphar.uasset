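; Lily pad (Nénuphar) actor whose Cube moves vertically between its placed position and a MoveZ offset.
; BeginPlay stores both positions and snaps the Cube to the offset one.
; The NenuUp event glides it back to the placed position over TimeForDown and clears Down.
; A timed MainCharacter-triggered down-and-up cycle is present but disconnected, and the overlap and Tick events do nothing.
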(event `self.ReceiveBeginPlay`
  (bind _cube (`self.Cube`))
  (bind (_posstart_x _posstart_y _posstart_z) (`KismetMathLibrary.BreakVector` (`self.PosStart`)))
  (set `self.PosStart` (`SceneComponent.RelativeLocation` _cube))
  (bind _output_get (set `self.PosEnd` (`KismetMathLibrary.MakeVector` _posstart_x _posstart_y (+ _posstart_z (`self.MoveZ`)))))
  (`SceneComponent.K2_SetRelativeLocation` _cube _output_get false false))

(event `self.ReceiveActorBeginOverlap`
  (params (OtherActor :type "Actor Object Reference")))

(event `self.ReceiveTick`
  (params (DeltaSeconds :type "Float (single-precision)"))
  (if (`self.Down`)
    _))

(event `NenuUp`
  (`KismetSystemLibrary.MoveComponentTo` (`self.Cube`) (`self.PosStart`) (struct) false false (`self.TimeForDown`))
  (set `self.Down` false))

(fn `UserConstructionScript`)