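; BP_Quenouille is an actor whose Quenouille component moves temporarily to an end position when the MainCharacter overlaps it.
; If the actor is down and the character has at least one Mana, overlap calls RegenElem, waits, then moves the component from StartPos toward EndPos.
; Tick polls IsUp and uses a latent Delay before moving the component back and clearing the flag.
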(event `self.ReceiveBeginPlay`
  (bind (_startpos_location _startpos_rotation) (`KismetMathLibrary.BreakTransform` (`self.StartPos`)))
  (`KismetSystemLibrary.MoveComponentTo` (`self.Quenouille`) _startpos_location _startpos_rotation))

(event `self.ReceiveActorBeginOverlap`
  (params (OtherActor :type "Actor Object Reference"))
  (bind (_endpos_location _endpos_rotation) (`KismetMathLibrary.BreakTransform` (`self.EndPos`)))
  (if (not (`self.IsUp`))
    (bind _asmain_character (cast `/Game/BluePrints/MainCharacter` OtherActor))
    (if (>= (`/Game/BluePrints/MainCharacter.Mana` _asmain_character) 1.0)
      (`/Game/BluePrints/MainCharacter.RegenElem` _asmain_character)
      (`KismetSystemLibrary.Delay` (`self.TimeBeforeMove`))
      (`KismetSystemLibrary.MoveComponentTo` (`self.Quenouille`) _endpos_location _endpos_rotation false false (`self.TimeForMove`))
      (set `self.IsUp` true))))

(event `self.ReceiveTick`
  (params (DeltaSeconds :type "Float (single-precision)"))
  (bind (_startpos_location _startpos_rotation) (`KismetMathLibrary.BreakTransform` (`self.StartPos`)))
  (if (`self.IsUp`)
    (`KismetSystemLibrary.Delay` (`self.TimeUp`))
    (`KismetSystemLibrary.MoveComponentTo` (`self.Quenouille`) _startpos_location _startpos_rotation false false (`self.TimeForMove`))
    (set `self.IsUp` false)))

(fn `UserConstructionScript`)