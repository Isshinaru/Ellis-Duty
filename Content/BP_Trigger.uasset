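; BP_Trigger is a trigger actor that shows tutorial text while the MainCharacter is inside its DialogueTrigger volume.
; On begin overlap it creates a UI_Tuto widget, passes Texte into Stringtuto and adds it to the viewport.
; On end overlap by the MainCharacter it removes the widget and clears the WidgetCreat guard against duplicates.
; That guard is set before the character cast, so any overlapping actor can set it.
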(event `self.ReceiveBeginPlay`)

(event `self.DialogueTrigger.OnComponentBeginOverlap`
  (params (OverlappedComponent :type "PrimitiveComponent Object Reference") (OtherActor :type "Actor Object Reference") (OtherComp :type "PrimitiveComponent Object Reference") (OtherBodyIndex :type Integer) (bFromSweep :type Boolean) (SweepResult :type "HitResult Structure (by ref)"))
  (if (not (`self.WidgetCreat?`))
    (set `self.WidgetCreat?` true)
    (cast `/Game/BluePrints/MainCharacter` OtherActor)
    (bind _returnvalue (`|CreateWidget` "/Game/UI_Tuto.UI_Tuto_C" (`GameplayStatics.GetPlayerController` 0)))
    (bind _output_get (set `self.TutoUMG` _returnvalue))
    (bind _output_get_2 (set `/Game/UI_Tuto.stringtuto` (`self.Texte`) _output_get))
    (`UserWidget.AddToViewport` _output_get 0)))

(event `self.DialogueTrigger.OnComponentEndOverlap`
  (params (OverlappedComponent :type "PrimitiveComponent Object Reference") (OtherActor :type "Actor Object Reference") (OtherComp :type "PrimitiveComponent Object Reference") (OtherBodyIndex :type Integer))
  (cast `/Game/BluePrints/MainCharacter` OtherActor)
  (set `self.WidgetCreat?` false)
  (`Widget.RemoveFromParent` (`self.TutoUMG`)))

(fn `UserConstructionScript`)