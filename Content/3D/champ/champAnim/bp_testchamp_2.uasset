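; Test mushroom actor (champ) that animates when the MainCharacter overlaps it, with a one-time regen state.
; Regen starts true, so the first overlap plays the regen animation on the skeletal mesh, swaps its material to red after a short delay, then clears the flag.
; Later overlaps play the jump (saut) animation.
; Only visuals are handled here, with no healing or launch logic.
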(event `self.ReceiveActorBeginOverlap`
  (params (OtherActor :type "Actor Object Reference"))
  (bind _champ3saut2_test (`self.champ3saut2_test`))
  (bind _champ3saut2_test_2 (`self.champ3saut2_test`))
  (cast `/Game/BluePrints/MainCharacter` OtherActor)
  (if (`self.regen?`)
    (`SkeletalMeshComponent.PlayAnimation` _champ3saut2_test "/Game/3D/champ/champAnim/champ3TestAnim3regen_Anim_Action.champ3TestAnim3regen_Anim_Action" false)
    (`SkeletalMeshComponent.Play` _champ3saut2_test false)
    (`KismetSystemLibrary.Delay` 0.6)
    (`PrimitiveComponent.SetMaterial` (`self.champ3saut2_test`) 0 "/Game/3D/champ/Mat_Rouge.Mat_Rouge")
    (set `self.regen?` false)
    (else
      (`SkeletalMeshComponent.PlayAnimation` _champ3saut2_test_2 "/Game/3D/champ/champAnim/champ3saut2_test_Anim_Action.champ3saut2_test_Anim_Action" false)
      (`SkeletalMeshComponent.Play` _champ3saut2_test_2 false))))

(event `self.Sphere.OnComponentBeginOverlap`
  (params (OverlappedComponent :type "PrimitiveComponent Object Reference") (OtherActor :type "Actor Object Reference") (OtherComp :type "PrimitiveComponent Object Reference") (OtherBodyIndex :type Integer) (bFromSweep :type Boolean) (SweepResult :type "HitResult Structure (by ref)")))

(event `self.ReceiveBeginPlay`
  (set `self.regen?` true))

(fn `UserConstructionScript`)