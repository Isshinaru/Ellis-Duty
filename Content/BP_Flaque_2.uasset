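; Water puddle actor that the MainCharacter absorbs on the Interaction input to refill Mana, capped at five.
; Box overlaps toggle a Detecte flag and a Gate that arms the input, while Bubble widgets show contextual prompts or fade.
; Each absorption sets TailleFlaque, calls AspireEau and draws down EnergieRegen; taking all of it destroys the puddle component and deactivates its particles.
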(event `InputAction|Interaction`
  (params (Key :type "Key Structure"))
  (bind _energieregen (`self.EnergieRegen`))
  (:`Pressed`
    (set `self.NoOverlap` true)
    (for _array_element (`PrimitiveComponent.GetOverlappingActors` (`self.Box`) null)
      (cast `/Game/BluePrints/MainCharacter` _array_element)
      (set `self.NoOverlap` false))
    (if (`self.NoOverlap`)
      _
      (elif (`/Game/BluePrints/MainCharacter.CanMove` (stale `self.Box.OnComponentBeginOverlap` _asmain_character))
        (if (< (`/Game/BluePrints/MainCharacter.Mana` (stale `self.Box.OnComponentBeginOverlap` _asmain_character)) 5.0)
          (`/Engine/EditorBlueprintResources/StandardMacros.Gate` true :!label _label
            (:`Exit`
              (bind _asmain_character (cast `/Game/BluePrints/MainCharacter` (stale `self.Box.OnComponentBeginOverlap` OtherActor)))
              (bind _returnvalue (- 5.0 (`/Game/BluePrints/MainCharacter.Mana` _asmain_character)))
              (bind _returnvalue_2 (`KismetMathLibrary.FMin` _returnvalue _energieregen))
              (if (== _returnvalue_2 _energieregen)
                (set `/Game/BluePrints/MainCharacter.TailleFlaque` _returnvalue_2 _asmain_character)
                (`/Game/BluePrints/MainCharacter.AspireEau` _asmain_character)
                (set `self.EnergieRegen` 0.0)
                (`ActorComponent.K2_DestroyComponent` (`self.Flaque`))
                (`ActorComponent.Deactivate` (`self.ParticleSystem`))
                (else
                  (bind _output_get (set `/Game/BluePrints/MainCharacter.TailleFlaque` _returnvalue _asmain_character))
                  (`/Game/BluePrints/MainCharacter.AspireEau` _asmain_character)
                  (set `self.EnergieRegen` (- _energieregen _output_get))))
              (bind _foundwidgets (`WidgetBlueprintLibrary.GetAllWidgetsOfClass` "/Game/BluePrints/UIWidgets/Bubble.Bubble_C"))
              (for _array_element_2 _foundwidgets
                (`/Game/BluePrints/UIWidgets/Bubble.Fade` _array_element_2))))
          (elif (> (`self.EnergieRegen`) 0.0)
            (bind _foundwidgets_2 (`WidgetBlueprintLibrary.GetAllWidgetsOfClass` "/Game/BluePrints/UIWidgets/Bubble.Bubble_C"))
            (for _array_element_3 _foundwidgets_2
              (`/Game/BluePrints/UIWidgets/Bubble.Bubulle` _array_element_3 3))))))))

(event `self.Box.OnComponentBeginOverlap`
  (params (OverlappedComponent :type "PrimitiveComponent Object Reference") (OtherActor :type "Actor Object Reference") (OtherComp :type "PrimitiveComponent Object Reference") (OtherBodyIndex :type Integer) (bFromSweep :type Boolean) (SweepResult :type "HitResult Structure (by ref)"))
  (bind _asmain_character (cast `/Game/BluePrints/MainCharacter` OtherActor))
  (if (`self.Detecte`)
    (set `self.Detecte` false)
    (if (> (`self.EnergieRegen`) 0.0)
      (bind _foundwidgets (`WidgetBlueprintLibrary.GetAllWidgetsOfClass` "/Game/BluePrints/UIWidgets/Bubble.Bubble_C"))
      (for _array_element _foundwidgets
        (`/Game/BluePrints/UIWidgets/Bubble.Bubulle` _array_element 0))
      (`self.EnableInput` (`GameplayStatics.GetPlayerController` 0))
      (goto _label :!via `Open`)
      (else
        (bind _foundwidgets_2 (`WidgetBlueprintLibrary.GetAllWidgetsOfClass` "/Game/BluePrints/UIWidgets/Bubble.Bubble_C"))
        (for _array_element_2 _foundwidgets_2
          (`/Game/BluePrints/UIWidgets/Bubble.Bubulle` _array_element_2 4))))))

(event `self.Box.OnComponentEndOverlap`
  (params (OverlappedComponent :type "PrimitiveComponent Object Reference") (OtherActor :type "Actor Object Reference") (OtherComp :type "PrimitiveComponent Object Reference") (OtherBodyIndex :type Integer))
  (set `self.NoOverlap` true)
  (for _array_element (`PrimitiveComponent.GetOverlappingActors` (`self.Box`) null)
    (cast `/Game/BluePrints/MainCharacter` _array_element)
    (set `self.NoOverlap` false))
  (if (`self.NoOverlap`)
    (if (not (`self.Detecte`))
      (set `self.Detecte` true)
      (bind _foundwidgets (`WidgetBlueprintLibrary.GetAllWidgetsOfClass` "/Game/BluePrints/UIWidgets/Bubble.Bubble_C"))
      (for _array_element_2 _foundwidgets
        (`/Game/BluePrints/UIWidgets/Bubble.Fade` _array_element_2))
      (goto _label :!via `Close`))))

(fn `UserConstructionScript`)