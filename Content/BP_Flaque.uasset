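; Puddle (flaque) that the main character can absorb once by pressing Interaction while inside its box.
; Overlap enables input, shows an E_Interaction prompt and opens a gate; leaving removes the prompt and closes the gate.
; A press flashes the prompt's pressed state; after a short delay, if the gate is open, it passes EnergieRegen to TailleFlaque, calls AspireEau and destroys the Flaque component.
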(event `self.ReceiveBeginPlay`)

(event `InputAction|Interaction`
  (params (Key :type "Key Structure"))
  (:`Pressed`
    (`KismetSystemLibrary.PrintString` "flaque")
    (set `/Game/E_Interaction.IsPressed` true (stale `self.Box.OnComponentBeginOverlap` _returnvalue))
    (`KismetSystemLibrary.Delay` 0.3)
    (set `/Game/E_Interaction.IsPressed` false (stale `self.Box.OnComponentBeginOverlap` _returnvalue))
    (`/Engine/EditorBlueprintResources/StandardMacros.Gate` true :!label _label
      (:`Exit`
        (`Widget.RemoveFromParent` (stale `self.Box.OnComponentBeginOverlap` _returnvalue))
        (if (`self.Up`)
          (bind _asmain_character (cast `/Game/BluePrints/MainCharacter` (stale `self.Box.OnComponentBeginOverlap` OtherActor)))
          (set `/Game/BluePrints/MainCharacter.TailleFlaque` (`self.EnergieRegen`) _asmain_character)
          (`/Game/BluePrints/MainCharacter.AspireEau` _asmain_character)
          (set `self.Up` false)
          (`ActorComponent.K2_DestroyComponent` (`self.Flaque`)))))))

(event `self.Box.OnComponentBeginOverlap`
  (params (OverlappedComponent :type "PrimitiveComponent Object Reference") (OtherActor :type "Actor Object Reference") (OtherComp :type "PrimitiveComponent Object Reference") (OtherBodyIndex :type Integer) (bFromSweep :type Boolean) (SweepResult :type "HitResult Structure (by ref)"))
  (`self.EnableInput` (`GameplayStatics.GetPlayerController` 0))
  (cast `/Game/BluePrints/MainCharacter` OtherActor)
  (if (`self.Detecte`)
    (set `self.Detecte` false)
    (`KismetSystemLibrary.PrintString` "begin")
    (bind _returnvalue (`|CreateWidget` "/Game/E_Interaction.E_Interaction_C"))
    (`UserWidget.AddToViewport` _returnvalue 0)
    (goto _label :!via `Open`)))

(event `self.Box.OnComponentEndOverlap`
  (params (OverlappedComponent :type "PrimitiveComponent Object Reference") (OtherActor :type "Actor Object Reference") (OtherComp :type "PrimitiveComponent Object Reference") (OtherBodyIndex :type Integer))
  (cast `/Game/BluePrints/MainCharacter` OtherActor)
  (if (not (`self.Detecte`))
    (set `self.Detecte` true)
    (`KismetSystemLibrary.PrintString` "end")
    (`Widget.RemoveFromParent` (stale `self.Box.OnComponentBeginOverlap` _returnvalue))
    (goto _label :!via `Close`)))

(fn `UserConstructionScript`)