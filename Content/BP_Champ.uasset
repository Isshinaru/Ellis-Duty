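; BP_Champ is an interactable jump pad that starts inactive until the player regenerates it with mana.
; Entering the Sphere shows an E_Interaction prompt, enables input and opens a Gate, which closes on exit.
; Interaction briefly flashes the prompt, then, given enough Mana, calls MainCharacter's RegenElem and sets IsRegen.
; Once regenerated, Box overlap passes JumpDir to MainCharacter and calls ChampJump.
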(event `self.ReceiveBeginPlay`)

(event `self.ReceiveActorBeginOverlap`
  (params (OtherActor :type "Actor Object Reference")))

(event `self.Box.OnComponentBeginOverlap`
  (params (OverlappedComponent :type "PrimitiveComponent Object Reference") (OtherActor :type "Actor Object Reference") (OtherComp :type "PrimitiveComponent Object Reference") (OtherBodyIndex :type Integer) (bFromSweep :type Boolean) (SweepResult :type "HitResult Structure (by ref)"))
  (`KismetSystemLibrary.PrintString` "Hello")
  (if (`self.IsRegen`)
    (bind _asmain_character (cast `/Game/BluePrints/MainCharacter` OtherActor))
    (set `/Game/BluePrints/MainCharacter.ChampJumpforce` (`self.JumpDir`) _asmain_character)
    (`/Game/BluePrints/MainCharacter.ChampJump` _asmain_character)))

(event `InputAction|Interaction`
  (params (Key :type "Key Structure"))
  (:`Pressed`
    (if (not (`self.IsRegen`))
      (set `/Game/E_Interaction.IsPressed` true (stale `self.Sphere.OnComponentBeginOverlap` _returnvalue))
      (`KismetSystemLibrary.Delay` 0.3)
      (set `/Game/E_Interaction.IsPressed` false (stale `self.Sphere.OnComponentBeginOverlap` _returnvalue))
      (`/Engine/EditorBlueprintResources/StandardMacros.Gate` true :!label _label
        (:`Exit`
          (bind _asmain_character (cast `/Game/BluePrints/MainCharacter` (stale `self.Sphere.OnComponentBeginOverlap` OtherActor)))
          (if (>= (`/Game/BluePrints/MainCharacter.Mana` _asmain_character) 1.0)
            (`Widget.RemoveFromParent` (stale `self.Sphere.OnComponentBeginOverlap` _returnvalue))
            (`/Game/BluePrints/MainCharacter.RegenElem` _asmain_character)
            (set `self.IsRegen` true)))))))

(event `self.Sphere.OnComponentBeginOverlap`
  (params (OverlappedComponent :type "PrimitiveComponent Object Reference") (OtherActor :type "Actor Object Reference") (OtherComp :type "PrimitiveComponent Object Reference") (OtherBodyIndex :type Integer) (bFromSweep :type Boolean) (SweepResult :type "HitResult Structure (by ref)"))
  (if (not (`self.IsRegen`))
    (`self.EnableInput` (`GameplayStatics.GetPlayerController` 0))
    (cast `/Game/BluePrints/MainCharacter` OtherActor)
    (if (`self.Detecte`)
      (set `self.Detecte` false)
      (`KismetSystemLibrary.PrintString` "begin")
      (bind _returnvalue (`|CreateWidget` "/Game/E_Interaction.E_Interaction_C"))
      (`UserWidget.AddToViewport` _returnvalue 0)
      (goto _label :!via `Open`))))

(event `self.Sphere.OnComponentEndOverlap`
  (params (OverlappedComponent :type "PrimitiveComponent Object Reference") (OtherActor :type "Actor Object Reference") (OtherComp :type "PrimitiveComponent Object Reference") (OtherBodyIndex :type Integer))
  (cast `/Game/BluePrints/MainCharacter` OtherActor)
  (if (not (`self.Detecte`))
    (set `self.Detecte` true)
    (`KismetSystemLibrary.PrintString` "end")
    (`Widget.RemoveFromParent` (stale `self.Sphere.OnComponentBeginOverlap` _returnvalue))
    (goto _label :!via `Close`)))

(event `self.Box.OnComponentEndOverlap`
  (params (OverlappedComponent :type "PrimitiveComponent Object Reference") (OtherActor :type "Actor Object Reference") (OtherComp :type "PrimitiveComponent Object Reference") (OtherBodyIndex :type Integer)))

(fn `UserConstructionScript`)