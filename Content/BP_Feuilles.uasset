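; An interactable leaves actor that the player can trigger once to call the character's RegenElem and slide three Feuille components along X.
; Box overlap shows an E_Interaction prompt widget and opens a gate for the Interaction input, and leaving removes and closes them.
; A press requires at least 1 Mana, sets a one-shot Regen flag, then after a delay runs MoveComponentTo toward targets computed at BeginPlay.
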(event `self.ReceiveBeginPlay`
  (bind (_relativelocation_x _relativelocation_y _relativelocation_z) (`KismetMathLibrary.BreakVector` (`SceneComponent.RelativeLocation` (`self.Feuille3`))))
  (bind (_relativelocation_x_2 _relativelocation_y_2 _relativelocation_z_2) (`KismetMathLibrary.BreakVector` (`SceneComponent.RelativeLocation` (`self.Feuille1`))))
  (bind (_relativelocation_x_3 _relativelocation_y_3 _relativelocation_z_3) (`KismetMathLibrary.BreakVector` (`SceneComponent.RelativeLocation` (`self.Feuille2`))))
  (set `self.MoveFeuille1` (`KismetMathLibrary.MakeVector` (+ _relativelocation_x_2 (`self.MoveX`)) _relativelocation_y_2 _relativelocation_z_2))
  (set `self.MoveFeuille2` (`KismetMathLibrary.MakeVector` (+ _relativelocation_x_3 (`self.MoveX`)) _relativelocation_y_3 _relativelocation_z_3))
  (set `self.MoveFeuille3` (`KismetMathLibrary.MakeVector` (+ _relativelocation_x (`self.MoveX`)) _relativelocation_y _relativelocation_z)))

(event `self.ReceiveActorBeginOverlap`
  (params (OtherActor :type "Actor Object Reference")))

(event `InputAction|Interaction`
  (params (Key :type "Key Structure"))
  (:`Pressed`
    (set `/Game/E_Interaction.IsPressed` true (stale `self.Box.OnComponentBeginOverlap` _returnvalue))
    (`KismetSystemLibrary.Delay` 0.3)
    (set `/Game/E_Interaction.IsPressed` false (stale `self.Box.OnComponentBeginOverlap` _returnvalue))
    (`/Engine/EditorBlueprintResources/StandardMacros.Gate` true :!label _label
      (:`Exit`
        (if (not (`self.Regen`))
          (bind _asmain_character (cast `/Game/BluePrints/MainCharacter` (stale `self.Box.OnComponentBeginOverlap` OtherActor)))
          (if (>= (`/Game/BluePrints/MainCharacter.Mana` _asmain_character) 1.0)
            (`Widget.RemoveFromParent` (stale `self.Box.OnComponentBeginOverlap` _returnvalue))
            (`/Game/BluePrints/MainCharacter.RegenElem` _asmain_character)
            (set `self.Regen` true)
            (`KismetSystemLibrary.Delay` (`self.TimeBefore`))
            (`KismetSystemLibrary.MoveComponentTo` (`self.Feuille1`) (`self.MoveFeuille1`) (struct) false false (`self.TimeFor`))
            (`KismetSystemLibrary.MoveComponentTo` (`self.Feuille2`) (`self.MoveFeuille2`) (struct) false false (`self.TimeFor`))
            (`KismetSystemLibrary.MoveComponentTo` (`self.Feuille3`) (`self.MoveFeuille3`) (struct) false false (`self.TimeFor`))))))))

(event `self.Box.OnComponentBeginOverlap`
  (params (OverlappedComponent :type "PrimitiveComponent Object Reference") (OtherActor :type "Actor Object Reference") (OtherComp :type "PrimitiveComponent Object Reference") (OtherBodyIndex :type Integer) (bFromSweep :type Boolean) (SweepResult :type "HitResult Structure (by ref)"))
  (if (not (`self.Regen`))
    (`self.EnableInput` (`GameplayStatics.GetPlayerController` 0))
    (cast `/Game/BluePrints/MainCharacter` OtherActor)
    (if (`self.Detecte`)
      (set `self.Detecte` false)
      (`KismetSystemLibrary.PrintString` "begin")
      (bind _returnvalue (`|CreateWidget` "/Game/E_Interaction.E_Interaction_C"))
      (`UserWidget.AddToViewport` _returnvalue 0)
      (goto _label :!via `Open`))))

(event `self.Box.OnComponentEndOverlap`
  (params (OverlappedComponent :type "PrimitiveComponent Object Reference") (OtherActor :type "Actor Object Reference") (OtherComp :type "PrimitiveComponent Object Reference") (OtherBodyIndex :type Integer))
  (cast `/Game/BluePrints/MainCharacter` OtherActor)
  (if (not (`self.Detecte`))
    (set `self.Detecte` true)
    (`KismetSystemLibrary.PrintString` "end")
    (`Widget.RemoveFromParent` (stale `self.Box.OnComponentBeginOverlap` _returnvalue))
    (goto _label :!via `Close`)))

(fn `UserConstructionScript`)