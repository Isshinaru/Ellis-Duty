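; BP_Arbre is an interactable tree that the main character regenerates once, moving its Tronc component from a start to an end position.
; Box overlap shows an E_Interaction prompt widget and opens a gate that lets the Interaction input through; leaving removes and closes them.
; Interacting with enough mana calls RegenElem on the character, sets Regen to block reuse, then after a delay animates the trunk with MoveComponentTo.
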(event `self.ReceiveBeginPlay`
  (bind (_startpos_location _startpos_rotation) (`KismetMathLibrary.BreakTransform` (`self.StartPos`)))
  (`KismetSystemLibrary.MoveComponentTo` (`self.Tronc`) _startpos_location _startpos_rotation))

(event `self.ReceiveActorBeginOverlap`
  (params (OtherActor :type "Actor Object Reference")))

(event `InputAction|Interaction`
  (params (Key :type "Key Structure"))
  (bind (_endpos_location _endpos_rotation) (`KismetMathLibrary.BreakTransform` (`self.EndPos`)))
  (:`Pressed`
    (if (not (`self.Regen`))
      (set `/Game/E_Interaction.IsPressed` true (stale `self.Box.OnComponentBeginOverlap` _returnvalue))
      (`KismetSystemLibrary.Delay` 0.3)
      (set `/Game/E_Interaction.IsPressed` false (stale `self.Box.OnComponentBeginOverlap` _returnvalue))
      (`/Engine/EditorBlueprintResources/StandardMacros.Gate` true :!label _label
        (:`Exit`
          (bind _asmain_character (cast `/Game/BluePrints/MainCharacter` (stale `self.Box.OnComponentBeginOverlap` OtherActor)))
          (if (>= (`/Game/BluePrints/MainCharacter.Mana` _asmain_character) 1.0)
            (`Widget.RemoveFromParent` (stale `self.Box.OnComponentBeginOverlap` _returnvalue))
            (`/Game/BluePrints/MainCharacter.RegenElem` _asmain_character)
            (set `self.Regen` true)
            (`KismetSystemLibrary.Delay` (`self.TimeBeforeUp`))
            (`KismetSystemLibrary.MoveComponentTo` (`self.Tronc`) _endpos_location _endpos_rotation false false (`self.TimeForUp`))))))))

(event `self.Box.OnComponentBeginOverlap`
  (params (OverlappedComponent :type "PrimitiveComponent Object Reference") (OtherActor :type "Actor Object Reference") (OtherComp :type "PrimitiveComponent Object Reference") (OtherBodyIndex :type Integer) (bFromSweep :type Boolean) (SweepResult :type "HitResult Structure (by ref)"))
  (if (not (`self.Regen`))
    (`self.EnableInput` (`GameplayStatics.GetPlayerController` 0))
    (cast `/Game/BluePrints/MainCharacter` OtherActor)
    (if (`self.Detecte`)
      (set `self.Detecte` false)
      (`KismetSystemLibrary.PrintString` "begin")
      (bind _returnvalue (`|CreateWidget` "/Game/E_Interaction.E_Interaction_C"))
      (`UserWidget.AddToViewport` _returnvalue 0)
      (goto _label :!via `Open`))))

(event `self.Box.OnComponentEndOverlap`
  (params (OverlappedComponent :type "PrimitiveComponent Object Reference") (OtherActor :type "Actor Object Reference") (OtherComp :type "PrimitiveComponent Object Reference") (OtherBodyIndex :type Integer))
  (cast `/Game/BluePrints/MainCharacter` OtherActor)
  (if (not (`self.Detecte`))
    (set `self.Detecte` true)
    (`KismetSystemLibrary.PrintString` "end")
    (`Widget.RemoveFromParent` (stale `self.Box.OnComponentBeginOverlap` _returnvalue))
    (goto _label :!via `Close`)))

(fn `UserConstructionScript`)